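; BP_TestNode is a test node actor that publishes an output direction and location and shows debug text about its link to a next node.
; Construction sets both outputs from the actor's own forward vector and location.
; Tick refreshes them, replacing the location's Z with the player character's, and prints its name joined to the next node's.
; The ActiveNode event prints the node's own name.
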(event EventBeginPlay)

(event Collision|EventActorBeginOverlap
  (params (OtherActor :type Actor%20Object%20Reference)))

(event EventTick
  (params (DeltaSeconds :type Float%20%28single-precision%29))
  (bind _returnvalue (Transformation|GetActorLocation))
  (Development|PrintString (Utilities|String|Append (Utilities|GetDisplayName self) "                          " (Utilities|GetDisplayName (Class|GamePlayNodeBase|GetNextNode))) true false "(R=0.000000,G=0.660000,B=1.000000,A=1.000000)" 0.0)
  (Variables|Default|SetOutDirectiron (Math|Vector|GetForwardVector (Transformation|GetActorRotation)))
  (Variables|Default|SetOutLocation (Math|Vector|MakeVector (.x _returnvalue) (.y _returnvalue) (.z (Transformation|GetActorLocation (Game|GetPlayerCharacter 0))))))

(event EventActiveNode
  (Development|PrintString (Utilities|String|Append "My name is : " (Utilities|GetDisplayName self))))

(fn ConstructionScript
  (Variables|Default|SetOutDirectiron (Math|Vector|GetForwardVector (Transformation|GetActorRotation)))
  (Variables|Default|SetOutLocation (Transformation|GetActorLocation)))